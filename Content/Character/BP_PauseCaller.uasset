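; BP_PauseCaller is an actor that toggles the pause menu when Escape is pressed.
; On BeginPlay it enables input from player controller 0 so it receives the key.
; Escape creates and shows a new pause menu widget, pauses the game, shows the cursor and switches to Game and UI input.
; If already paused, it removes the stored widget, unpauses, hides the cursor and restores game-only input.
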(event EventBeginPlay
  (Input|EnableInput (Game|GetPlayerController 0)))

(event Input|KeyboardEvents|Escape
  (params (Key :type Key%20Structure :default "None"))
  (bind _returnvalue (Game|GetPlayerController 0))
  (:Pressed
    (if (not (Game|IsGamePaused))
      (bind _returnvalue_2 (UserInterface|CreateWidget "/Game/UI/InGame/WB_PauseMenu.WB_PauseMenu_C"))
      (bind _output_get (Variables|Default|SetSpawnedWidget _returnvalue_2))
      (UserInterface|Viewport|AddtoViewport _output_get 0)
      (Game|SetGamePaused true)
      (Variables|/Script/Engine.PlayerController|SetbShowMouseCursor _returnvalue true)
      (Input|SetInputModeGameandUI _returnvalue 0 "DoNotLock" false false)
      (else
        (Widget|RemovefromParent (Variables|Default|GetSpawnedWidget))
        (Game|SetGamePaused false)
        (Variables|/Script/Engine.PlayerController|SetbShowMouseCursor _returnvalue false)
        (Input|SetInputModeGameOnly _returnvalue false)))))

(fn ConstructionScript)