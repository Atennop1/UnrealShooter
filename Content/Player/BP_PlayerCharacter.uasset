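; BP_PlayerCharacter is the player character Blueprint, assembled from separate components for movement, crouching, rotation, aiming, jumping, health and weapon handling.
; Its construction script assigns each component to a matching variable, likely inherited from a parent class.
; It also wires dependencies between them: rotation receives the camera, shooting receives the recoil component, and dying receives a point to attach the camera after death.
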(fn ConstructionScript
  (Utilities|FlowControl|Sequence
    (:then_0
      (Variables|Default|SetMovingComponent (Variables|Default|GetCharacterMoving)))
    (:then_1
      (Variables|Default|SetCrouchingComponent (Variables|Default|GetCharacterCrouching)))
    (:then_2
      (bind _output_get (Variables|Default|SetRotatingComponent (Variables|Default|GetCharacterRotating)))
      (Variables|/Script/UnrealShooter.CharacterRotatingComponent|SetCharacterCamera _output_get (Variables|Default|GetCamera)))
    (:then_3
      (Variables|Default|SetWeaponHoldingComponent (Variables|Default|GetCharacterWeaponHolding)))
    (:then_4
      (Variables|Default|SetAimingComponent (Variables|Default|GetCharacterAiming)))
    (:then_5
      (Variables|Default|SetWeaponThrowingComponent (Variables|Default|GetCharacterWeaponThrowing)))
    (:then_6
      (bind _output_get_2 (Variables|Default|SetShootingComponent (Variables|Default|GetCharacterShooting)))
      (Variables|/Script/UnrealShooter.CharacterShootingComponent|SetRecoilingComponent _output_get_2 (Variables|Default|GetCharacterWeaponRecoiling)))
    (:then_7
      (Variables|Default|SetReloadingComponent (Variables|Default|GetCharacterReloading)))
    (:then_8
      (Variables|Default|SetHealth (Variables|Default|GetCharacterHealth))
      (Variables|/Script/UnrealShooter.CharacterDyingComponent|SetComponentToAttachCamera (Variables|Default|GetCharacterDying) (Variables|Default|GetPlaceToCameraAfterDeath)))
    (:then_9
      (Variables|Default|SetJumpingComponent (Variables|Default|GetCharacterJumping)))))